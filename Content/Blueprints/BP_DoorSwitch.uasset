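; BP_DoorSwitch is a one-way switch that can be flipped only after all of its referenced collectibles are activated.
; It binds to each collectible's activation event, gathering activated ones into a unique array and comparing its length to the full list.
; Once unlocked, interaction sets the state to Activated, broadcasts SwitchEnabled and plays a timeline that lerps the switch from its current position toward MoveLocation.
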(event `self.ReceiveBeginPlay`
  (for _array_element (`self.CollectibleRef`)
    (add `/Game/Blueprints/BP_Collectible.OnCollectibleActivated` _array_element (delegate `CheckSwitchStatus`))))

(event `CheckSwitchStatus`
  (for _array_element (`self.CollectibleRef`)
    (if (`|EnumEquality` (`/Game/Blueprints/BP_Collectible.CurrentState` _array_element) "NewEnumerator1")
      (`KismetArrayLibrary.Array_AddUnique` (`self.ActivatedCollectible`) _array_element)))
  (if (== (`KismetArrayLibrary.Array_Length` (`self.CollectibleRef`)) (`KismetArrayLibrary.Array_Length` (`self.ActivatedCollectible`)))
    (set `self.AllCollectiblesActivated` true)))

(event `/Game/Blueprints/BPI_Interactable.TriggerInteraction`
  (if (`self.AllCollectiblesActivated`)
    (switch `/Game/Blueprints/E_Activateable` (`self.CurrentState`)
      (:`NewEnumerator0`
        (set `self.CurrentState` "NewEnumerator1")
        (`self.FlipSwitch`)
        (`self.SwitchEnabled`)))))

(event `FlipSwitch`
  (bind _switch (`self.Switch`))
  (bind (_direction _slideswitch) (`Timeline|SlideSwitch`)
    (:`Update`
      (`SceneComponent.K2_SetWorldLocation` _switch (`KismetMathLibrary.VLerp` (`SceneComponent.K2_GetComponentLocation` _switch) (`SceneComponent.K2_GetComponentLocation` (`self.MoveLocation`)) _slideswitch) false false))))

(fn `UserConstructionScript`)