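; Game instance that owns the save data and tracks how many puzzle pressure plates have been activated.
; Init loads BP_MySaveData from the default slot, or creates and saves a new one if none exists.
; IncrementKeyCount raises a runtime counter and calls SavePuzzleData, which is an empty stub, as is GetSavedGameData.
; SavePlayerData_1 separately increments the saved plate total and writes it to the slot.
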(event `self.ReceiveInit`
  (bind _returnvalue (`GameplayStatics.DoesSaveGameExist` (`self.DefaultSaveSlot`)))
  (if _returnvalue
    (bind _returnvalue_2 (`GameplayStatics.LoadGameFromSlot` (`self.DefaultSaveSlot`)))
    (bind _asbp_my_save_data (cast `/Game/Blueprints/BP_MySaveData` _returnvalue_2))
    (set `self.SaveGameData` _asbp_my_save_data)
    (`KismetSystemLibrary.PrintString` (`KismetStringLibrary.Concat_StrStr` "Game loaded, total pressure plates:" (`KismetStringLibrary.Conv_IntToString` (`/Game/Blueprints/BP_MySaveData.SavedTotalPressurePlatesActivated` _asbp_my_save_data))))
    (else
      (bind _returnvalue_3 (`GameplayStatics.CreateSaveGameObject` "/Game/Blueprints/BP_MySaveData.BP_MySaveData_C"))
      (bind _output_get (set `self.SaveGameData` _returnvalue_3))
      (`GameplayStatics.SaveGameToSlot` _output_get (`self.DefaultSaveSlot`)))))

(event `IncrementKeyCount`
  (bind _result (`/Engine/EditorBlueprintResources/StandardMacros.IncrementInt` (`self.TotalPressurePlatesActivated`))
    (:`  `
      (`KismetSystemLibrary.PrintString` (`KismetStringLibrary.Conv_IntToString` _result))
      (`/Game/Blueprints/BPI_SaveGame.SavePuzzleData`))))

(event `SavePlayerData_1`
  (bind _savegamedata (`self.SaveGameData`))
  (`/Engine/EditorBlueprintResources/StandardMacros.IncrementInt` (`/Game/Blueprints/BP_MySaveData.SavedTotalPressurePlatesActivated` _savegamedata)
    (:`  `
      (`GameplayStatics.SaveGameToSlot` _savegamedata (`self.DefaultSaveSlot`)))))

(fn `GetSavedGameData`
  (returns (SaveDataObject :type "/Game/Blueprints/BP_MySaveData Object Reference"))
  (return null))

(fn `SavePuzzleData`)