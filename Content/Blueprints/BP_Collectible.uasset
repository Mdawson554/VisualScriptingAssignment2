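; BP_Collectible is a collectible actor that reacts once to an interaction while it is deactivated.
; On begin play it copies the saved collectible total from the Game Instance's save data into CollectedAmount.
; TriggerInteraction switches the state to Activated, fires the OnCollectibleActivated dispatcher, starts a Niagara effect and applies a lit dynamic material to the mesh.
; The total is not incremented here, and the closing delay leads to nothing.
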(event `self.ReceiveBeginPlay`
  (bind _savedataobject (message `/Game/Blueprints/BPI_SaveGame.GetSavedGameData` (`GameplayStatics.GetGameInstance`)))
  (set `self.CollectedAmount` (`/Game/Blueprints/BP_MySaveData.SavedTotalCollectibles` _savedataobject)))

(event `/Game/Blueprints/BPI_Interactable.TriggerInteraction`
  (switch `/Game/Blueprints/E_Activateable` (`self.CurrentState`)
    (:`NewEnumerator0`
      (`|ExecutionSequence`
        (:`then_0`
          (set `self.CurrentState` "NewEnumerator1")
          (`self.OnCollectibleActivated`))
        (:`then_1`
          (`ActorComponent.Activate` (`self.Niagara`) false))
        (:`then_2`
          (`self.collectColourSurge`)
          (`KismetSystemLibrary.Delay` 0.5))))))

(fn `collectColourSurge`
  (`PrimitiveComponent.CreateDynamicMaterialInstance` (`self.Collectible`) 0 "/Game/Materials/M_LightActivated.M_LightActivated" "None"))

(fn `UserConstructionScript`)