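; BP_Door is a sliding door that opens once all of its referenced pressure plates have been activated.
; On BeginPlay it binds to each plate's activation event, then rechecks all plates whenever one fires, adding those in the required state to a list that is never cleared.
; When that list matches the plate count, a timeline lerps the door mesh from its current world location toward the MoveLocation component.
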(event `self.ReceiveBeginPlay`
  (for _array_element (`self.PressurePlateRef`)
    (add `/Game/Blueprints/BP_PressurePlate.OnPressurePlateActivated` _array_element (delegate `CheckDoorStatus`))))

(event `CheckDoorStatus`
  (for _array_element (`self.PressurePlateRef`)
    (if (`|EnumEquality` (`/Game/Blueprints/BP_PressurePlate.CurrentState` _array_element) "NewEnumerator1")
      (`KismetArrayLibrary.Array_AddUnique` (`self.ActivatedPlates`) _array_element)))
  (if (== (`KismetArrayLibrary.Array_Length` (`self.PressurePlateRef`)) (`KismetArrayLibrary.Array_Length` (`self.ActivatedPlates`)))
    (`self.OpenDoor`)))

(event `OpenDoor`
  (bind _sliding_door (`self.sliding door`))
  (bind (_direction _slidedoor) (`Timeline|slidedoor`)
    (:`Update`
      (`SceneComponent.K2_SetWorldLocation` _sliding_door (`KismetMathLibrary.VLerp` (`SceneComponent.K2_GetComponentLocation` _sliding_door) (`SceneComponent.K2_GetComponentLocation` (`self.MoveLocation`)) _slidedoor) false false))))

(fn `UserConstructionScript`)