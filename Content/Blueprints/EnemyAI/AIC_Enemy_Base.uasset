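; Base enemy AI controller that runs BT_Enemy_Base and turns perception into blackboard state.
; On possess it seeds the player as target and sets engagement distance; BeginPlay caches all patrol points.
; Sight updates set or clear the player target, saving the last stimulus location for investigation when sight is lost.
; The noise handler compares against AISenseConfig_Hearing, not the sense class, and would store the receiver's location, not the noise's.
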(event `self.ReceiveBeginPlay`
  (bind _outactors (`GameplayStatics.GetAllActorsOfClass` "/Game/Blueprints/EnemyAI/BP_PatrolPoint.BP_PatrolPoint_C"))
  (set `self.PatrolPoints` _outactors))

(event `self.ReceivePossess`
  (params (PossessedPawn :type "Pawn Object Reference"))
  (bind _returnvalue (`AIBlueprintHelperLibrary.GetBlackboard` null))
  (`self.RunBehaviorTree` "/Game/Blueprints/EnemyAI/BT_Enemy_Base.BT_Enemy_Base")
  (`KismetSystemLibrary.Delay` 0.2)
  (`BlackboardComponent.SetValueAsObject` _returnvalue (`self.Target Name`) (`GameplayStatics.GetPlayerCharacter` 0))
  (`BlackboardComponent.SetValueAsFloat` _returnvalue (`self.Target Distance Name`) (`self.Engagement Distance`)))

(event `self.AIPerception.OnTargetPerceptionUpdated`
  (params (Actor :type "Actor Object Reference") (Stimulus :type "AIStimulus Structure"))
  (`self.HandleSightStimulus` Actor Stimulus)
  (`self.HandleNoiseStimulus` Actor Stimulus)
  (`KismetSystemLibrary.PrintString` (`KismetSystemLibrary.GetDisplayName` Actor)))

(fn `HandleNoiseStimulus`
  (params (PercievedActor :type "Actor Object Reference") (Stimulus :type "AIStimulus Structure"))
  (bind (_stimulus_age _stimulus_expirationage _stimulus_strength _stimulus_stimuluslocation _stimulus_receiverlocation) (break `AIStimulus` (`local.Stimulus`)))
  (bind _returnvalue (`AIPerceptionSystem.GetSenseClassForStimulus` Stimulus))
  (if (== _returnvalue "/Script/AIModule.AISenseConfig_Hearing")
    (`BlackboardComponent.SetValueAsVector` (`AIBlueprintHelperLibrary.GetBlackboard` null) (`self.InvestigationTargetName`) _stimulus_receiverlocation)
    (else
      (return))))

(fn `HandleSightStimulus`
  (params (PercievedActor :type "Actor Object Reference") (Stimulus :type "AIStimulus Structure"))
  (bind _returnvalue (`AIBlueprintHelperLibrary.GetBlackboard` null))
  (bind (_stimulus_age _stimulus_expirationage _stimulus_strength _stimulus_stimuluslocation _stimulus_receiverlocation _stimulus_tag _stimulus_bsuccessfullysensed) (break `AIStimulus` (`local.Stimulus`)))
  (bind _investigationtargetname (`self.InvestigationTargetName`))
  (bind _returnvalue_2 (`AIPerceptionSystem.GetSenseClassForStimulus` Stimulus))
  (if (== _returnvalue_2 "/Script/AIModule.AISense_Sight")
    (if (== (`local.PercievedActor`) (`GameplayStatics.GetPlayerCharacter` 0))
      (`BlackboardComponent.SetValueAsObject` (`AIBlueprintHelperLibrary.GetBlackboard` null) (`self.Target Name`) (`KismetMathLibrary.SelectObject` (`GameplayStatics.GetPlayerCharacter` 0) null _stimulus_bsuccessfullysensed))
      (if _stimulus_bsuccessfullysensed
        (`BlackboardComponent.ClearValue` _returnvalue _investigationtargetname)
        (else
          (`BlackboardComponent.SetValueAsVector` _returnvalue _investigationtargetname _stimulus_stimuluslocation)))
      (else
        (return)))
    (else
      (return))))

(fn `UserConstructionScript`)