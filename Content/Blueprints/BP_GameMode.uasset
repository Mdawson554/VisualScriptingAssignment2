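; Game mode for a pressure plate puzzle that tracks activated plates and handles the win.
; On BeginPlay it caches the player's BP_PlatformingCharacter.
; IncreasePressurePlateCount increments the count and, when it hits the target, marks the puzzle complete, stops the character, disables input and shows the W_WinPrompt widget.
; It then triggers DelayTime, which waits briefly before opening Lvl_ThirdPerson.
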(event `self.ReceiveBeginPlay`
  (bind _asbp_platforming_character (cast `/Game/Variant_Platforming/Blueprints/BP_PlatformingCharacter` (`GameplayStatics.GetPlayerPawn` 0)))
  (set `self.AsPlatformingCharachter` _asbp_platforming_character))

(event `DelayTime`
  (`KismetSystemLibrary.Delay` 3.0)
  (`GameplayStatics.OpenLevelBySoftObjectPtr` "/Game/ThirdPerson/Lvl_ThirdPerson.Lvl_ThirdPerson"))

(fn `IncreasePressurePlateCount`
  (bind _returnvalue (`GameplayStatics.GetPlayerController` 0))
  (bind _asplatformingcharachter (`self.AsPlatformingCharachter`))
  (bind _result (`/Engine/EditorBlueprintResources/StandardMacros.IncrementInt` (`self.PressurePlatesActivated`))
    (:`  `
      (if (== _result (`self.PressurePlatesToWin`))
        (set `self.IsPuzzleCompelte` true)
        (`MovementComponent.StopMovementImmediately` (`Pawn.GetMovementComponent` _asplatformingcharachter))
        (`self.DisableInput` _asplatformingcharachter _returnvalue)
        (set `self.Message To Display` "")
        (bind _returnvalue_2 (`|CreateWidget` "/Game/Blueprints/UI/W_WinPrompt.W_WinPrompt_C" _returnvalue))
        (`UserWidget.AddToViewport` _returnvalue_2 0)
        (`self.DelayTime`)))))

(fn `UserConstructionScript`)