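; BP_LightSwitch is a light indicator that switches on when its referenced pressure plate is activated.
; On BeginPlay it binds to the plate's activation dispatcher.
; Activation applies a dynamic instance of the activated material to the light and plays a sound through a DoOnce gate.
; It then sets IsLightActivated and fires its own OnLightActivated dispatcher for other listeners.
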(event `self.ReceiveBeginPlay`
  (add `/Game/Blueprints/BP_PressurePlate.OnPressurePlateActivated` (`self.PressurePlateRef`) (delegate `ColourChange`)))

(event `ColourChange`
  (`self.LightColourChange`)
  (set `self.isLightActivated` true)
  (`self.OnLightActivated`))

(fn `LightColourChange`
  (bind _sfxplayer (`self.SFXPlayer`))
  (`PrimitiveComponent.CreateDynamicMaterialInstance` (`self.Light`) 0 "/Game/Materials/M_LightActivated.M_LightActivated" "None")
  (`/Engine/EditorBlueprintResources/StandardMacros.DoOnce` false
    (:`Completed`
      (`AudioComponent.SetSound` _sfxplayer (`self.SFXToPlay`))
      (`AudioComponent.Play` _sfxplayer 0.0))))

(fn `UserConstructionScript`)